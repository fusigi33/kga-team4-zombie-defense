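; BP_Timer is a countdown actor that pauses the game when its time limit runs out.
; A looping one-second timer started on BeginPlay calls DecreaseTime, which decrements TimeLeft.
; At zero it clears the timer and pauses the game; the nodes that would create and show the game-over widget are disabled.
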(event `self.ReceiveBeginPlay`
  (`KismetSystemLibrary.K2_SetTimer` null "DecreaseTime" 1.0 true))

(fn `DecreaseTime`
  ; 매 초마다 시간 차감
  (bind _result (`/Engine/EditorBlueprintResources/StandardMacros.DecrementInt` (`self.TimeLeft`))
    (:`  `
      (bind _output_get (set `self.TimeLeft` _result))
      ; 제한 시간이 지나면 게임 오버 UI를 출력하고 일시정지
      (if (<= _output_get 0)
        (`KismetSystemLibrary.K2_ClearTimer` null "DecreaseTime")
        (bind _returnvalue (`|CreateWidget` null :!enabledstate Disabled))
        (`UserWidget.AddToViewport` _returnvalue 0 :!enabledstate Disabled)
        (`GameplayStatics.SetGamePaused` true)))))

(fn `UserConstructionScript`)