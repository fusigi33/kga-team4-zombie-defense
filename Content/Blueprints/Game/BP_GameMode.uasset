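; Game mode for a round-based zombie survival game with a time limit per round.
; A looping one-second timer drains time once the target map is entered; timeout or player death loses.
; Zombie deaths decrement a counter that advances the round and resets the time, winning after the final round.
; SpawnZombies staggers spawns across random BP_ZombieSpawner actors; GameOver pauses the game, with win/lose widgets currently disabled.
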(event `self.ReceiveBeginPlay`
  (`KismetSystemLibrary.K2_SetTimer` null "DecreaseTime" 1.0 true))

(event `OnZombieDeath`
  ; 좀비가 죽을 때마다 카운트 1 감소
  (bind _result (`/Engine/EditorBlueprintResources/StandardMacros.DecrementInt` (`self.RemainingZombieCount`))
    (:`  `
      (if (<= _result 0)
        ; 좀비가 없으면 다음 라운드 진입
        (`self.GoToNextRound`)))))

(event `OnPlayerDeath`
  (`self.GameOver` false))

(event `SpawnZombies`
  ; 월드에 있는 BP_ZombieSpawner에서 랜덤으로 좀비 생성
  (bind _outactors (`GameplayStatics.GetAllActorsOfClass` "/Game/Blueprints/Game/BP_ZombieSpawner.BP_ZombieSpawner_C"))
  (set `self.ZombieSpawners` _outactors)
  (for _ (range (+ (`|GetArrayItem` (`self.ZombiesPerRound`) (`self.Round`)) 1))
    (`/Game/Blueprints/Game/BP_ZombieSpawner.SpawnZombie` (`|GetArrayItem` (`self.ZombieSpawners`) (`KismetMathLibrary.RandomInteger` (`KismetArrayLibrary.Array_Length` (`self.ZombieSpawners`)))))
    (`KismetSystemLibrary.Delay` 0.2)))

(fn `DecreaseTime`
  ; 플레이어가 좀비 맵에 진입했는지 확인
  (if (`self.bIsInTargetMap`)
    ; 매 초마다 시간 차감
    (`KismetSystemLibrary.PrintString` (`KismetStringLibrary.Conv_IntToString` (`self.TimeLeft` :!enabledstate Disabled) :!enabledstate Disabled) :!enabledstate Disabled)
    (bind _result (`/Engine/EditorBlueprintResources/StandardMacros.DecrementInt` (`self.TimeLeft`))
      (:`  `
        (bind _output_get (set `self.TimeLeft` _result))
        (if (<= _output_get 0)
          ; 시간이 초과되면 게임 오버
          (`self.GameOver` false))))))

(fn `GameOver`
  (params (bIsPlayerWinner :type Boolean))
  ; 게임 오버 UI를 출력하고 일시정지
  (`KismetSystemLibrary.K2_ClearTimer` null "DecreaseTime")
  (if (`local.bIsPlayerWinner`)
    ;; Player Win UI 출력
    (bind _returnvalue (`|CreateWidget` null :!enabledstate Disabled))
    (`UserWidget.AddToViewport` _returnvalue 0 :!enabledstate Disabled)
    (else
      ;; Player Lose UI 출력
      (bind _returnvalue_2 (`|CreateWidget` null :!enabledstate Disabled))
      (`UserWidget.AddToViewport` _returnvalue_2 0 :!enabledstate Disabled)))
  (`GameplayStatics.SetGamePaused` true))

(fn `GoToNextRound`
  (if (< (`self.Round`) (`self.MaxRound`))
    ; 라운드가 남아 있을 경우 다음 라운드 진입
    (`/Engine/EditorBlueprintResources/StandardMacros.IncrementInt` (`self.Round`)
      (:`  `
        ; 제한 시간 할당
        (set `self.TimeLeft` (`|GetArrayItem` (`self.RoundTimes`) (- (`self.Round`) 1)))))
    (else
      ; 승리
      (`self.GameOver` true))))

(fn `UserConstructionScript`)